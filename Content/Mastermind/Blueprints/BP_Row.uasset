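; BP_Row is a row actor for a Mastermind game, holding four spheres.
; On BeginPlay it gathers the four spheres into the RowSpheres array in a fixed order.
; A click on the actor is passed on by calling Clicked, with no other logic in this graph.
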(event `self.ReceiveBeginPlay`
  (bind _rowspheres (`self.RowSpheres`))
  (`KismetArrayLibrary.Array_Add` _rowspheres (`self.Sphere`))
  (`KismetArrayLibrary.Array_Add` _rowspheres (`self.Sphere1`))
  (`KismetArrayLibrary.Array_Add` _rowspheres (`self.Sphere2`))
  (`KismetArrayLibrary.Array_Add` _rowspheres (`self.Sphere3`)))

(event `self.ReceiveActorOnClicked`
  (params (ButtonPressed :type "Key Structure"))
  (`self.Clicked`))

(fn `UserConstructionScript`)